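; Base gun Blueprint that handles firing in semi, three-round burst and full-auto modes.
; A shot needs a chambered round: it spawns the bullet, muzzle effect and ejected casing at component transforms and plays the firing sound.
; Each shot then calls Load, which spends ammo and delays by fire rate before re-chambering.
; Looping timers drive burst and auto fire, while the delayed bullet-destroy range limit is unconnected.
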(event `self.ReceiveBeginPlay`
  ;[1 1 1] 游戏开始自动上膛
  (`self.Load`))

(event `Load`
  ;[1 1 1] 子弹上膛
  (if (> (`self.Ammo`) 0)
    (`/Engine/EditorBlueprintResources/StandardMacros.DecrementInt` (`self.Ammo`)
      (:`  `
        (`KismetSystemLibrary.Delay` (/ 1.0 (`self.FireRate`)))
        (set `self.BulletInBore` true)))
    (else
      (set `self.BulletInBore` false))))

(event `FirstSingleBullet`
  (bind _returnvalue (`SceneComponent.K2_GetComponentToWorld` (`self.BarrelArrow`)))
  ;[1 1 1] 发射单发子弹
  (if (`self.BulletInBore`)
    (bind _returnvalue_2 (`|SpawnActorFromClass` (`self.BulletClass`) _returnvalue "Undefined" "OverrideRootScale" null null))
    (set `self.Bullet` _returnvalue_2)
    (set `self.BulletLocation` (.location _returnvalue))
    (`|ExecutionSequence`
      (:`then_0`
        ;;[1 1 1] 开火音效
        (`GameplayStatics.PlaySoundAtLocation` (`self.FiringSound`) (`self.BulletLocation`) (struct) 1.0 1.0 0.0 null null null))
      (:`then_1`
        ;;[1 1 1] 开火枪口特效
        (`|SpawnActorFromClass` (`self.MuzzleClass`) (`SceneComponent.K2_GetComponentToWorld` (`self.FlashRoot`)) "Undefined" "OverrideRootScale" null null))
      (:`then_2`
        ;;[1 1 1] 抛出弹壳
        (`|SpawnActorFromClass` (`self.CartridgeClass`) (`SceneComponent.K2_GetComponentToWorld` (`self.EjectorArrow`)) "Undefined" "OverrideRootScale" null null))
      (:`then_3`
        ;;[1 1 1] 通过重新上膛控制射击速度
        (`self.Load`)))))

(event `Fire`
  ;[1 1 1] 开火
  (switch `/Game/Gun/FireModeEnum` (`self.FireMode`)
    (:`NewEnumerator0`
      ;;[1 1 1] 单发
      (`self.FirstSingleBullet`))
    (:`NewEnumerator1`
      ;;[1 1 1] 三连发
      (bind _returnvalue (`KismetSystemLibrary.K2_SetTimerDelegate` (delegate `BurstFire`) (/ 10.0 (`self.FireRate`)) true)))
    (:`NewEnumerator2`
      ;;[1 1 1] 全自动
      (bind _returnvalue_2 (`KismetSystemLibrary.K2_SetTimerDelegate` (delegate `AutoFire`) (/ 1.0 (`self.FireRate`)) true)))))

(event `BurstFire`
  ;[1 1 1] 开火
  ;;[1 1 1] 三连发
  (if (> (`self.BurstCount`) 0)
    (`self.FirstSingleBullet`)
    (`/Engine/EditorBlueprintResources/StandardMacros.DecrementInt` (`self.BurstCount`))
    (else
      (`KismetSystemLibrary.K2_ClearAndInvalidateTimerHandle` (stale `Fire` _returnvalue))
      (set `self.BurstCount` 3))))

(event `CeaseAutoFire`
  ;[1 1 1] 开火
  ;;[1 1 1] 全自动
  (`KismetSystemLibrary.K2_ClearAndInvalidateTimerHandle` (stale `Fire` _returnvalue_2)))

(event `AutoFire`
  ;[1 1 1] 开火
  ;;[1 1 1] 全自动
  (if (> (`self.Ammo`) 0)
    (`self.FirstSingleBullet`)))

(fn `UserConstructionScript`)