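; Gatling gun child Blueprint that adds barrel spin-up, motor audio and an ammo counter widget to its parent gun.
; Fire starts a BarrelRotate timeline that drives Tick-based barrel spin and squared-rate motor pitch, calling parent fire only once the forward spin-up finishes.
; CeaseAutoFire reverses the timeline to spin down and stop the motor sound.
; The widget's bullet count is set at BeginPlay and in FirstSingleBullet.
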(event `self.ReceiveBeginPlay`
  ;[1 1 1] 子弹数UI
  (`parent.ReceiveBeginPlay`)
  (bind _returnvalue (`|CreateWidget` "/Game/UI/MainUI/BulletUI_Gatlin.BulletUI_Gatlin_C"))
  (bind _output_get (set `self.BulletUI` _returnvalue))
  (set `/Game/UI/MainUI/BulletUI_Gatlin.BulletCount` (`self.Ammo`) _output_get)
  (`UserWidget.AddToViewport` (`self.BulletUI`) 0))

(event `self.FirstSingleBullet`
  ;[1 1 1] 子弹数UI
  (`parent.FirstSingleBullet`)
  (set `/Game/UI/MainUI/BulletUI_Gatlin.BulletCount` (`self.Ammo`) (`self.BulletUI`)))

(event `self.ReceiveTick`
  (params (DeltaSeconds :type "Float (single-precision)"))
  ;[1 1 1] 重写开火事件
  (`parent.ReceiveTick` DeltaSeconds)
  (`/Engine/EditorBlueprintResources/StandardMacros.Gate` true :!label _label
    (:`Exit`
      ;;[1 1 1] 枪口旋转
      (`SceneComponent.K2_AddLocalRotation` (`self.BarrelGatlin`) (`KismetMathLibrary.MakeRotator` (`self.RotateRate`)) false false))))

(event `self.Fire`
  ;[1 1 1] 重写开火事件
  (`AudioComponent.Play` (`self.FiringAudio`) 0.0)
  (set `self.FireRate` 15.0)
  (set `self.FiringSound` "/Game/Weapon/SFX/miniSoundCue.miniSoundCue")
  (`|ExecutionSequence`
    (:`then_0`
      (goto _label :!via `Open`))
    (:`then_1`
      (bind (_direction _rotatecoefficient) (`Timeline|BarrelRotate` :!label _label_2)
        (:`Update`
          (bind _output_get (set `self.RotateRate` (* _rotatecoefficient 50.0)))
          ;;[1 1 1] 使用转速调节电机音调
          (`AudioComponent.SetPitchMultiplier` (`self.FiringAudio`) (`KismetMathLibrary.MapRangeClamped` (`KismetMathLibrary.Square` _output_get) 0.0 1.0 0.1 2.0)))
        (:`Finished`
          ;;[1 1 1] 转速达到最快后才开始触发父类开火事件
          (if (`|EnumEquality` _direction "Forward")
            (`parent.Fire`)
            (else
              (`AudioComponent.Stop` (`self.FiringAudio`)))))))))

(event `self.CeaseAutoFire`
  ;[1 1 1] 重写开火事件
  ;;[1 1 1] 重写熄火事件
  (`|ExecutionSequence`
    (:`then_0`
      (goto _label_2 :!via `Reverse`))
    (:`then_1`
      (`parent.CeaseAutoFire`))))

(fn `UserConstructionScript`
  (`parent.UserConstructionScript`))