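; 75CM gun Blueprint that extends a parent gun with an ammo counter widget and animated barrel recoil.
; On BeginPlay it creates the BulletUI_75CM widget, seeds it with Ammo and adds it to the viewport.
; FirstSingleBullet runs parent logic, then refreshes the count.
; The overridden Load (chambering) event restarts the Rebound timeline, which offsets the barrel mesh along local X, before calling the parent Load.
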(event `self.ReceiveBeginPlay`
  ;[1 1 1] 子弹数UI
  (`parent.ReceiveBeginPlay`)
  (bind _returnvalue (`|CreateWidget` "/Game/UI/MainUI/BulletUI_75CM.BulletUI_75CM_C"))
  (bind _output_get (set `self.BulletUI` _returnvalue))
  (set `/Game/UI/MainUI/BulletUI_75CM.BulletCount` (`self.Ammo`) _output_get)
  (`UserWidget.AddToViewport` (`self.BulletUI`) 0))

(event `self.FirstSingleBullet`
  ;[1 1 1] 子弹数UI
  (`parent.FirstSingleBullet`)
  (set `/Game/UI/MainUI/BulletUI_75CM.BulletCount` (`self.Ammo`) (`self.BulletUI`)))

(event `self.ReceiveTick`
  (params (DeltaSeconds :type "Float (single-precision)"))
  ;[1 1 1] 重写上膛事件枪管动态效果
  (`parent.ReceiveTick` DeltaSeconds))

(event `self.Load`
  ;[1 1 1] 重写上膛事件枪管动态效果
  (`|ExecutionSequence`
    (:`then_0`
      (bind (_direction _reboundcoefficient) (`Timeline|Rebound` :!via `PlayFromStart`)
        (:`Update`
          (`SceneComponent.K2_SetRelativeLocation` (`self.Barrel75CM`) (`KismetMathLibrary.MakeVector` (* _reboundcoefficient -30.0)) false false))))
    (:`then_1`
      (`parent.Load`))))

(fn `UserConstructionScript`
  (`parent.UserConstructionScript`))